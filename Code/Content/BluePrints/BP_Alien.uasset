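; BP_Alien is an alien actor that displays a health bar through a widget component.
; Every Tick it rotates the bar toward the player camera, using a look-at rotation computed from the actor's location.
; The same update casts the widget to WBP_HealthBar and sets its progress bar to Vie divided by MaxHealth.
; The graph only reads health and contains no damage or movement logic.
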(event `self.ReceiveTick`
  (params (DeltaSeconds :type "Float (single-precision)"))
  (`self.updateLifeBar`))

(event `updateLifeBar`
  ; LifeBar
  (`SceneComponent.K2_SetWorldRotation` (`self.HealthBar`) (`KismetMathLibrary.FindLookAtRotation` (`self.K2_GetActorLocation`) (`self.K2_GetActorLocation` (`GameplayStatics.GetPlayerCameraManager` 0))) false false)
  (bind _aswbp_health_bar (cast `/Game/UI/WBP_HealthBar` (`WidgetComponent.GetWidget` (`self.HealthBar`))))
  (`ProgressBar.SetPercent` (`/Game/UI/WBP_HealthBar.ProgressBar_0` _aswbp_health_bar) (/ (`self.Vie`) (`self.MaxHealth`))))

(fn `UserConstructionScript`)